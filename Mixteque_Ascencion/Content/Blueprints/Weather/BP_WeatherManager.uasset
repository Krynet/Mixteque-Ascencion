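; Weather manager that runs the day/night clock, world temperature and random weather.
; Tick advances elapsed time to rotate the directional light, update the sky sphere and send the clock to the HUD.
; A looping timer derives temperature from a daily curve, setting Snow or Rain flags.
; Delayed random checks toggle player precipitation particles and timelines driving fog density, sun dimming, and snow/wetness in a material parameter collection.
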(event `self.ReceiveBeginPlay`
  (`|ExecutionSequence`
    (:`then_0`
      (`self.GetSunAndSky`))
    (:`then_1`
      (`self.SetSunIntensity`))
    (:`then_2`
      (`self.SetElapsedTime`))
    (:`then_3`
      (`self.StartUpdatingTemp`))))

(event `StartFog`
  (`KismetSystemLibrary.Delay` 3.0)
  (bind (_direction _fogdensity) (`Timeline|FogDensity` :!label _label)
    (:`Update`
      (`ExponentialHeightFogComponent.SetFogDensity` (`ExponentialHeightFog.Component` (`self.Fog`)) _fogdensity))))

(event `ReverseFog`
  (`KismetSystemLibrary.Delay` 3.0)
  (goto _label :!via `Reverse`))

(event `self.ReceiveTick`
  (params (DeltaSeconds :type "Float (single-precision)"))
  (`|ExecutionSequence`
    (:`then_0`
      (`self.UpdateElapsedTime`))
    (:`then_1`
      (`self.UpdateSunPosition`))
    (:`then_2`
      (`self.SetHUDRef`))
    (:`then_3`
      (`self.FadeSun`))
    (:`then_4`
      (`self.UpdateCurrentTime`))
    (:`then_5`
      (`KismetSystemLibrary.Delay` (`self.WeatherCheck`))
      (`self.SetWeather`))
    (:`then_6`
      (if (`self.Foggy?`)
        (bind (_direction _sunintensity _sunvisibility) (`Timeline|SunSettings` :!label _label_2)
          (:`Update`
            (`LightComponent.SetIntensity` (`Light.LightComponent` (`self.Sun`)) _sunintensity)
            (`MeshComponent.SetScalarParameterValueOnMaterials` (`/Engine/EngineSky/BP_Sky_Sphere.SkySphereMesh` (`self.Sky`)) "Sun brightness" _sunvisibility)))
        (else
          (goto _label_2 :!via `Reverse`))))))

(event `StartSnowCover`
  (`KismetSystemLibrary.Delay` 7.0)
  (bind (_direction _snowamount) (`Timeline|SnowCover` :!label _label_3)
    (:`Update`
      (`KismetMaterialLibrary.SetScalarParameterValue` "/Game/Blueprints/Weather/Materials/SnowCover/MPC_Weather.MPC_Weather" "SnowAmount" _snowamount))))

(event `ReverseSnowCover`
  (`KismetSystemLibrary.Delay` 14.0)
  (goto _label_3 :!via `Reverse`))

(event `StartWetness`
  (`KismetSystemLibrary.Delay` 7.0)
  (bind (_direction _wetness) (`Timeline|Timeline_0` :!label _label_4)
    (:`Update`
      (`KismetMaterialLibrary.SetScalarParameterValue` "/Game/Blueprints/Weather/Materials/SnowCover/MPC_Weather.MPC_Weather" "Wetness" _wetness))))

(event `ReverseWetness`
  (`KismetSystemLibrary.Delay` 14.0)
  (goto _label_4 :!via `Reverse`))

(fn `DetermineCurrentTime`
  (returns (Time :type "/Game/Blueprints/Weather/Data/S_Time Structure"))
  (bind _returnvalue (`self.GetFractionDay`))
  (return (make `/Game/Blueprints/Weather/Data/S_Time` (`KismetMathLibrary.FTrunc` (* (mod _returnvalue 1.0) 24.0)) (`KismetMathLibrary.FTrunc` (mod (* _returnvalue 1440.0) 60.0)))))

(fn `DetermineNight`
  (returns (ReturnValue :type Boolean))
  (bind _currenttime_hours (break `/Game/Blueprints/Weather/Data/S_Time` (`self.CurrentTime`)))
  (return (or (< _currenttime_hours (`self.SunUpTime`)) (>= _currenttime_hours (`self.SunDownTime`)))))

(fn `FadeSun`
  (bind _lightcomponent (`Light.LightComponent` (`self.Sun`)))
  (`LightComponent.SetIntensity` _lightcomponent (`KismetMathLibrary.FClamp` (+ (`LightComponentBase.Intensity` _lightcomponent) (* (`GameplayStatics.GetWorldDeltaSeconds`) (/ 24.0 (`self.SecondsPerDay`)) (`self.SunIntensity`) (select `bool` (`self.DetermineNight`) :!type "Float (single-precision)"))) 0.0 (`self.SunIntensity`))))

(fn `GetFractionDay`
  (returns (ReturnValue :type "Float (double-precision)"))
  (return (/ (`self.ElapsedTime`) (`self.SecondsPerDay`))))

(fn `GetSunAndSky`
  (`/Engine/EditorBlueprintResources/StandardMacros.IsValid` (`self.Sun`)
    (:`Is Valid`
      _)
    (:`Is Not Valid`
      (bind _outactors (`GameplayStatics.GetAllActorsOfClass` "/Script/Engine.DirectionalLight"))
      (set `self.Sun` (`|GetArrayItem` _outactors))))
  (`/Engine/EditorBlueprintResources/StandardMacros.IsValid` (`self.Sky`)
    (:`Is Valid`
      (`/Engine/EditorBlueprintResources/StandardMacros.IsValid` (stale _output_get)
        (:`Is Not Valid`
          (bind _outactors_2 (`GameplayStatics.GetAllActorsOfClass` "/Script/Engine.ExponentialHeightFog"))
          (set `self.Fog` (`|GetArrayItem` _outactors_2)))))
    (:`Is Not Valid`
      (bind _outactors_3 (`GameplayStatics.GetAllActorsOfClass` "/Engine/EngineSky/BP_Sky_Sphere.BP_Sky_Sphere_C"))
      (bind _output_get (set `self.Sky` (`|GetArrayItem` _outactors_3))))))

(fn `GetTimeAsSeconds`
  (params (Time :type "/Game/Blueprints/Weather/Data/S_Time Structure"))
  (returns (ReturnValue :type Integer))
  (bind (_hours _minutes) (break `/Game/Blueprints/Weather/Data/S_Time` Time))
  (return (+ (* _hours 3600) (* _minutes 60))))

(fn `SetElapsedTime`
  (set `self.ElapsedTime` (* (`self.GetTimeAsSeconds` (`self.StartTime`)) (/ (`self.SecondsPerDay`) 86400.0))))

(fn `SetHUDRef`
  (`/Engine/EditorBlueprintResources/StandardMacros.IsValid` (`self.HUDRef`)
    (:`Is Not Valid`
      (bind _asmy_player (cast `/Game/Blueprints/Character/My_Player` (`GameplayStatics.GetPlayerCharacter` 0)))
      (set `self.HUDRef` (`/Game/Blueprints/Character/My_Player.GameHUDRef` _asmy_player)))))

(fn `SetSunIntensity`
  (set `self.SunIntensity` (`LightComponentBase.Intensity` (`Light.LightComponent` (`self.Sun`)))))

(fn `SetWeather`
  (bind _asmy_player (cast `/Game/Blueprints/Character/My_Player` (`GameplayStatics.GetPlayerCharacter` 0)))
  (if (`KismetMathLibrary.RandomBool`)
    (if (`KismetMathLibrary.RandomBool`)
      (`self.StartFog`)
      (set `self.Foggy?` true)
      (else
        (`self.ReverseFog`)
        (set `self.Foggy?` false)))
    (bind _output_get (set `self.Precipitation?` (`KismetMathLibrary.RandomBool`)))
    (if _output_get
      (if (`self.Snow?`)
        (`ActorComponent.Activate` (`/Game/Blueprints/Character/My_Player.PS_Snow` _asmy_player) false)
        (`self.StartSnowCover`)
        (elif (`self.Rain?`)
          (bind _ps_rain (`/Game/Blueprints/Character/My_Player.PS_Rain` _asmy_player))
          (`ActorComponent.Activate` _ps_rain false)
          (`self.StartWetness`)
          (set `self.IsRain?` true)
          (else
            (`ActorComponent.Deactivate` _ps_rain :!label _label)
            (`self.ReverseSnowCover`)
            (`self.ReverseWetness`)
            (`self.ReverseFog`)
            (set `self.IsRain?` false)
            (set `self.Foggy?` false))))
      (else
        (goto _label)))
    (else
      (goto _label))))

(fn `StartUpdatingTemp`
  (`KismetSystemLibrary.K2_SetTimer` self "UpdateWorldTemperature" (/ 1.0 (`self.TemperatureUpdateRate`)) true))

(fn `UpdateCurrentTime`
  (bind _output_get (set `self.CurrentTime` (`self.DetermineCurrentTime`)))
  (`/Game/Blueprints/Weather/HUD_Time.SetTime` (`self.HUDRef`) _output_get (`self.ClockType`)))

(fn `UpdateElapsedTime`
  (set `self.ElapsedTime` (+ (`self.ElapsedTime`) (`GameplayStatics.GetWorldDeltaSeconds`))))

(fn `UpdateSunPosition`
  (`SceneComponent.K2_SetRelativeRotation` (`Light.LightComponent` (`self.Sun`)) (`KismetMathLibrary.MakeRotator` 0.0 (+ (* (`self.GetFractionDay`) -360.0) 90.0) 40.0) false false)
  (`/Engine/EngineSky/BP_Sky_Sphere.UpdateSunDirection` (`self.Sky`)))

(fn `UpdateWorldTemperature`
  (bind _output_get (set `self.FinalWorldTemperature` (+ (* (`CurveFloat.GetFloatValue` (`self.TemperatureFluctuation`) (mod (`self.GetFractionDay`) 1.0)) (`self.WorldTemperatureVariation`)) (`self.BaseWorldTemperature`))))
  (if (< _output_get 5.0)
    (set `self.Snow?` true)
    (else
      (set `self.Rain?` true)))
  (`/Game/Blueprints/Weather/HUD_Time.SetWorldTemp` (`self.HUDRef`) _output_get (`self.DegreeType`)))

(fn `UserConstructionScript`
  (set `self.SecondsPerDay` (* (`self.MinutesPerDay`) 60.0)))